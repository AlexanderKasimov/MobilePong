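; BP_PlayerPaddle is a player paddle actor that holds itself to a fixed X position and a target height.
; On BeginPlay it sets TargetLocation from the SpawnLocation of BPObjectType.
; Each Tick it makes a swept move to the constant X and the target Z, keeping its current Y.
; No input handling appears in this graph, and the construction script only calls its parent.
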(event EventBeginPlay
  (Variables|Default|SetTargetLocation (Variables|/Game/Blueprints/BP_ObjectType.BP_ObjectType_C|GetSpawnLocation (Variables|Default|GetBP_ObjectType))))

(event EventTick
  (params (DeltaSeconds :type Float%20%28single-precision%29))
  (Transformation|SetActorLocation (Math|Vector|MakeVector 15.0 (.Y (Math|Vector|BreakVector (Transformation|GetActorLocation))) (.Z (Math|Vector|BreakVector (Variables|Default|GetTargetLocation)))) true false))

(fn ConstructionScript
  (|CallParentFunction))