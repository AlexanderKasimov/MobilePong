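; Pong game mode that runs an AI-versus-AI menu backdrop and 1 Player matches against an AI paddle.
; StartMenu and Start1P clear the board, spawn paddles and set the player controller's mode.
; PaddleScored respawns the menu ball or updates scores, then starts another round with briefly blocked input or shows the winner.
; Named timers delay ball spawns and raise ball speed up to a capped step count each round.
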(event EventBeginPlay
  (bind _asbp_pong_player_controller (Utilities|Casting|CastToBP_PongPlayerController (Game|GetPlayerController 0)))
  (Variables|Default|SetPlayerControllerRef _asbp_pong_player_controller)
  (CallFunction|StartMenu))

(fn ConstructionScript)

(fn SpawnBall
  (bind _returnvalue (Game|SpawnActorfromClass "/Game/Blueprints/BP_Ball.BP_Ball_C" (Math|Transform|MakeTransform "15.000000, 0, 0" "0, 0, 0" "0.062500,0.062500,0.062500") "Undefined" 0 (Math|Vector|MakeVector 0.0 (select (Math|Random|RandomBool) 1.0 -1.0) (Math|Random|RandomFloatinRange (* (Variables|Default|GetMaxRespawnAngle) -1.0) (Variables|Default|GetMaxRespawnAngle))) 0))
  (Variables|Default|SetBallRef _returnvalue))

(fn PaddleScored
  (params (isLeftBorder? :type Boolean))
  (switch Utilities|FlowControl|Switch|SwitchonEnum_PlayMode (Variables|Default|GetPlayMode)
    (:NewEnumerator0
      (Utilities|Time|SetTimerbyFunctionName 0 "SpawnBall" (Variables|Default|GetBallRespawnTime)))
    (:NewEnumerator1
      (Utilities|FlowControl|Sequence
        (:then_0
          (if isLeftBorder?
            (Math|Integer|IncrementInt (Variables|Default|GetRightPlayerScore))
            (else
              (Math|Integer|IncrementInt (Variables|Default|GetLeftPlayerScore)))))
        (:then_1
          (if (CallFunction|ShouldEndMatch?)
            (CallFunction|EndMatch)
            (else
              (CallFunction|BlockInput)
              (CallFunction|SetUnblockInputTimer)
              (CallFunction|StartRound))))))))

(fn ShouldEndMatch?
  (return (or (>= (Variables|Default|GetLeftPlayerScore) (Variables|Default|GetScoreLimit)) (>= (Variables|Default|GetRightPlayerScore) (Variables|Default|GetScoreLimit)))))

(fn ResetScores
  (Variables|Default|SetLeftPlayerScore 0)
  (Variables|Default|SetRightPlayerScore 0))

(fn SetWinScreenText
  (CallFunction|SetWinner)
  (switch Utilities|FlowControl|Switch|SwitchonEnum_PlayMode (Variables|Default|GetPlayMode)
    (:NewEnumerator1
      (Variables|Default|SetWinnerText (select (Variables|Default|GetisLeftPlayerWin?) "AI WIN" "PLAYER WIN")))
    (:NewEnumerator2
      (Variables|Default|SetWinnerText (select (Variables|Default|GetisLeftPlayerWin?) "PLAYER 2" "PLAYER 1")))))

(fn StartGame
  (CallFunction|ResetScores)
  (CallFunction|StartRound))

(fn SetWinner
  (Variables|Default|SetisLeftPlayerWin? (> (Variables|Default|GetLeftPlayerScore) (Variables|Default|GetRightPlayerScore))))

(fn RestartGame)

(fn SpawnSecondPaddle(D)
  (bind _outactors (Actor|GetAllActorsOfClass (Variables|Default|GetPaddleTypeToSpawn)))
  (if (== (Utilities|Array|Length _outactors) 0)
    (bind _returnvalue (Game|SpawnActorfromClass (Variables|Default|GetPaddleTypeToSpawn) (Math|Transform|MakeTransform "15.000000,-520.000000,0.000000") "Undefined" 0 0))
    (Utilities|Casting|CastToBP_PaddlePawn _returnvalue)
    (elif (and (.bSuccess (Utilities|Casting|CastToBP_PaddlePawn (Utilities|Array|Get(acopy) _outactors))) (< (Utilities|Array|Length _outactors) 2))
      (bind _returnvalue_2 (Game|SpawnActorfromClass (Variables|Default|GetPaddleTypeToSpawn) (Math|Transform|MakeTransform "15.000000,-460.000000,0.000000") "Undefined" 0 0))
      (bind _asbp_paddle_pawn (Utilities|Casting|CastToBP_PaddlePawn _returnvalue_2))
      (Utilities|Casting|CastToBP_PongPlayerController (Game|GetPlayerController 0)))))

(fn SpeedUpBall
  (Utilities|IsValid (Variables|Default|GetBallRef)
    (:Is%20Valid
      (bind _result (Math|Integer|IncrementInt (Variables|Default|GetCurBallSpeedUpCount))
        (:%20%20
          (if (< _result (Variables|Default|GetMaxBallSpeedUpCount))
            (Variables|/Game/Blueprints/BP_Ball.BP_Ball_C|SetVelocity (Variables|Default|GetBallRef) (+ (Variables|/Game/Blueprints/BP_Ball.BP_Ball_C|GetVelocity (Variables|Default|GetBallRef)) (Variables|Default|GetBallSpeedUpAmount)))
            (else
              (CallFunction|ResetBallSpeedUpTimer))))))))

(fn SetBallSpeedUpTimer
  (Variables|Default|SetCurBallSpeedUpCount 0)
  (CallFunction|ResetBallSpeedUpTimer)
  (bind _returnvalue (Utilities|Time|SetTimerbyFunctionName 0 "SpeedUpBall" (Variables|Default|GetBallSpeedUpInterval) true))
  (Variables|Default|SetBallSpeedUpTimerHandle _returnvalue))

(fn ResetBallSpeedUpTimer
  (Utilities|Time|ClearandInvalidateTimerbyHandle (Variables|Default|GetBallSpeedUpTimerHandle)))

(fn StartRound
  (bind _returnvalue (Utilities|Time|SetTimerbyFunctionName 0 "SpawnBall" (Variables|Default|GetBallRespawnTime)))
  (Variables|Default|SetSpawnBallTimerHandle _returnvalue)
  (CallFunction|SetBallSpeedUpTimer))

(fn RecenterPaddles
  (bind _outactors (Actor|GetAllActorswithTag "Paddle"))
  (for _array_element _outactors
    (bind _asbp_paddle_pawn (Utilities|Casting|CastToBP_PaddlePawn _array_element)
      (:then
        (Default|Recenter _asbp_paddle_pawn))
      (:CastFailed
        (Transformation|SetActorLocation _array_element (Variables|/Game/Blueprints/BP_ObjectType.BP_ObjectType_C|GetSpawnLocation (Actor|GetComponentbyClass _array_element "/Game/Blueprints/BP_ObjectType.BP_ObjectType_C")) false false)))))

(fn SetUnblockInputTimer
  (Utilities|Time|SetTimerbyFunctionName 0 "UnBlockInput" 1.0))

(fn BlockInput
  (bind _asbp_pong_player_controller (Utilities|Casting|CastToBP_PongPlayerController (Game|GetPlayerController 0)))
  (Default|BlockInput _asbp_pong_player_controller))

(fn UnBlockInput
  (bind _asbp_pong_player_controller (Utilities|Casting|CastToBP_PongPlayerController (Game|GetPlayerController 0)))
  (Default|UnBlockInput _asbp_pong_player_controller))

(fn SpawnAIforMenu
  (bind _returnvalue (Game|SpawnActorfromClass "/Game/Blueprints/BP_AiPaddle.BP_AiPaddle_C" (Math|Conversions|ToTransform(Vector) (Variables|Default|GetLeftSpawnLocation)) "Undefined" 0 0))
  (Variables|/Game/Blueprints/BP_ObjectType.BP_ObjectType_C|SetSpawnLocation (Variables|/Game/Blueprints/BP_BasePaddle.BP_BasePaddle_C|GetBP_ObjectType _returnvalue) (Variables|Default|GetLeftSpawnLocation))
  (bind _returnvalue_2 (Game|SpawnActorfromClass "/Game/Blueprints/BP_AiPaddle.BP_AiPaddle_C" (Math|Conversions|ToTransform(Vector) (Variables|Default|GetRightSpawnLocation)) "Undefined" 0 0))
  (Variables|/Game/Blueprints/BP_ObjectType.BP_ObjectType_C|SetSpawnLocation (Variables|/Game/Blueprints/BP_BasePaddle.BP_BasePaddle_C|GetBP_ObjectType _returnvalue_2) (Variables|Default|GetRightSpawnLocation)))

(fn StartMenu
  (CallFunction|ClearBoard)
  (CallFunction|SpawnAIforMenu)
  (Default|SetMenuMode (Variables|Default|GetPlayerControllerRef))
  (Variables|Default|SetPlayMode "NewEnumerator0")
  (CallFunction|SpawnBall))

(fn Start1P
  (CallFunction|ClearBoard)
  (CallFunction|Spawnfor1P)
  (Variables|/Game/Blueprints/BP_PongPlayerController.BP_PongPlayerController_C|SetRightPlayerRef (Variables|Default|GetPlayerControllerRef) (Variables|Default|GetRightPlayerRef))
  (Default|Set1PMode (Variables|Default|GetPlayerControllerRef))
  (Variables|Default|SetPlayMode "NewEnumerator1")
  (CallFunction|StartGame))

(fn Spawnfor1P
  (Utilities|FlowControl|Sequence
    (:then_0
      (bind _returnvalue (Game|SpawnActorfromClass "/Game/Blueprints/BP_AiPaddle.BP_AiPaddle_C" (Math|Conversions|ToTransform(Vector) (Variables|Default|GetLeftSpawnLocation)) "Undefined" 0 0))
      (bind _output_get (LocalVariables|SetAiPaddleRef _returnvalue))
      (Variables|/Game/Blueprints/BP_AiPaddle.BP_AiPaddle_C|SetMinSpeed _output_get (Variables|Default|GetAiMinSpeed))
      (Variables|/Game/Blueprints/BP_AiPaddle.BP_AiPaddle_C|SetMaxSpeed (LocalVariables|GetAiPaddleRef) (Variables|Default|GetAiMaxSpeed))
      (Variables|/Game/Blueprints/BP_ObjectType.BP_ObjectType_C|SetSpawnLocation (Variables|/Game/Blueprints/BP_BasePaddle.BP_BasePaddle_C|GetBP_ObjectType (LocalVariables|GetAiPaddleRef)) (Variables|Default|GetLeftSpawnLocation)))
    (:then_1
      (bind _returnvalue_2 (Game|SpawnActorfromClass "/Game/Blueprints/BP_PlayerPaddle.BP_PlayerPaddle_C" (Math|Conversions|ToTransform(Vector) (Variables|Default|GetRightSpawnLocation)) "Undefined" 0 0))
      (bind _output_get_2 (Variables|Default|SetRightPlayerRef _returnvalue_2))
      (Variables|/Game/Blueprints/BP_ObjectType.BP_ObjectType_C|SetSpawnLocation (Variables|/Game/Blueprints/BP_BasePaddle.BP_BasePaddle_C|GetBP_ObjectType _output_get_2) (Variables|Default|GetRightSpawnLocation)))))

(fn ClearBoard
  (Utilities|FlowControl|Sequence
    (:then_0
      (bind _outactors (Actor|GetAllActorsOfClass "/Game/Blueprints/BP_BasePaddle.BP_BasePaddle_C"))
      (for _array_element _outactors
        (Actor|DestroyActor _array_element)))
    (:then_1
      (bind _outactors_2 (Actor|GetAllActorsOfClass "/Game/Blueprints/BP_Ball.BP_Ball_C"))
      (for _array_element_2 _outactors_2
        (Actor|DestroyActor _array_element_2)))
    (:then_2
      (CallFunction|ClearSpawnBallTimer))))

(fn EndMatch
  (CallFunction|SetWinScreenText)
  (Default|SetWinScreenMode (Variables|Default|GetPlayerControllerRef) (Variables|Default|GetWinnerText)))

(fn ClearSpawnBallTimer
  (Utilities|Time|ClearandInvalidateTimerbyHandle (Variables|Default|GetSpawnBallTimerHandle)))