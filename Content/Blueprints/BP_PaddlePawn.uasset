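; Paddle pawn with a Paper2D sprite that creates the gameplay UI widget and moves only along the vertical axis.
; BeginPlay stores the spawn point in BPObjectType as the initial target, which the Recenter event restores.
; Tick snaps height to TargetLocation with a swept move, pinning X and preserving Y.
; MoveUp input is an empty deprecated event, and the touch-tracking, stepped-movement and debug-print nodes are disconnected.
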(event Custom|Recenter
  (Variables|Default|SetTargetLocation (Variables|/Game/Blueprints/BP_ObjectType.BP_ObjectType_C|GetSpawnLocation (Variables|Default|GetBP_ObjectType))))

(event EventBeginPlay
  (bind _returnvalue (UserInterface|CreateWidget "/Game/UI/UI_GameplayWidget.UI_GameplayWidget_C"))
  (UserInterface|Viewport|AddtoViewport _returnvalue 0)
  (bind _output_get (Variables|/Game/Blueprints/BP_ObjectType.BP_ObjectType_C|SetSpawnLocation (Variables|Default|GetBP_ObjectType) (Transformation|GetActorLocation)))
  (Variables|Default|SetTargetLocation _output_get))

(event EventTick
  (params (DeltaSeconds :type Float%20%28single-precision%29))
  (Transformation|SetActorLocation (Math|Vector|MakeVector 15.0 (.Y (Math|Vector|BreakVector (Transformation|GetActorLocation))) (.Z (Math|Vector|BreakVector (Variables|Default|GetTargetLocation)))) true false))

(event Input|AxisEvents|InputAxisMoveUp
  (params (AxisValue :type Float%20%28single-precision%29))
  ;[1 0 0.0313] Deprecated
)

(event Input|TouchEvents|InputTouch
  (params (Location :type Vector) (FingerIndex :type ETouchIndex%20Enum))
  ;[1 0 0.0313] Deprecated
)

(fn ConstructionScript
  (Transformation|SetRelativeRotation (Variables|Default|GetPaperSprite) "0,90.000000, 0" false false))