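; AI-controlled paddle for a Pong-style game that moves vertically along Z to track the ball.
; Each Tick it picks a direction and does a swept move, chasing the ball while it is on the paddle's half (Y sign), otherwise returning to spawn height.
; An Accuracy dead zone stops movement near the target, and a looping timer periodically randomises Speed within a range to vary its play.
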(event EventBeginPlay
  (Utilities|Time|SetTimerbyFunctionName 0 "UpdateSpeed" 4.0 true))

(event Collision|EventActorBeginOverlap
  (params (OtherActor :type Actor%20Object%20Reference)))

(event EventTick
  (params (DeltaSeconds :type Float%20%28single-precision%29))
  (CallFunction|UpdateDirection)
  (Transformation|SetActorLocation (+ (* (Variables|Default|GetDirection) (* (Variables|Default|GetSpeed) (Utilities|Time|GetWorldDeltaSeconds))) (Transformation|GetActorLocation)) true false))

(fn ConstructionScript
  (|CallParentFunction))

(fn UpdateSpeed
  (Variables|Default|SetSpeed (Math|Random|RandomFloatinRange (Variables|Default|GetMinSpeed) (Variables|Default|GetMaxSpeed))))

(fn ShouldMove?
  (if (> (.Y (Math|Vector|BreakVector (Variables|/Game/Blueprints/BP_ObjectType.BP_ObjectType_C|GetSpawnLocation (Variables|Default|GetBP_ObjectType)))) 0.0)
    (return (> (.Y (Math|Vector|BreakVector (Transformation|GetActorLocation (Variables|Default|GetBallRef)))) 0.0))
    (else
      (return (< (.Y (Math|Vector|BreakVector (Transformation|GetActorLocation (Variables|Default|GetBallRef)))) 0.0)))))

(fn UpdateDirection
  (bind _returnvalue (Transformation|GetActorLocation))
  (bind _ballref (Variables|Default|GetBallRef))
  (bind _returnvalue_2 (Transformation|GetActorLocation _ballref))
  (bind _z (Math|Vector|BreakVector _returnvalue))
  (bind _z_2 (Math|Vector|BreakVector _returnvalue_2))
  (bind _returnvalue_3 (- _z_2 _z))
  (Utilities|IsValid (Variables|Default|GetBallRef)
    (:Is%20Valid
      (if (CallFunction|ShouldMove?)
        (if (> (Math|Float|Absolute(Float) _returnvalue_3) (Variables|Default|GetAccuracy))
          (Variables|Default|SetDirection (Math|Vector|MakeVector 0.0 0.0 (Math|Float|Sign(Float) _returnvalue_3)))
          (else
            (Variables|Default|SetDirection "0, 0, 0")))
        (else
          (CallFunction|MovetoCenter))))
    (:Is%20Not%20Valid
      (CallFunction|MovetoCenter))))

(fn MovetoCenter
  (bind _returnvalue (Transformation|GetActorLocation))
  (bind _bp_objecttype (Variables|Default|GetBP_ObjectType))
  (bind _z (Math|Vector|BreakVector _returnvalue))
  (bind _spawnlocation (Variables|/Game/Blueprints/BP_ObjectType.BP_ObjectType_C|GetSpawnLocation _bp_objecttype))
  (bind _z_2 (Math|Vector|BreakVector _spawnlocation))
  (bind _returnvalue_2 (- _z_2 _z))
  (if (> (Math|Float|Absolute(Float) _returnvalue_2) (Variables|Default|GetAccuracy))
    (Variables|Default|SetDirection (Math|Vector|MakeVector 0.0 0.0 (Math|Float|Sign(Float) _returnvalue_2)))
    (else
      (Variables|Default|SetDirection "0, 0, 0"))))