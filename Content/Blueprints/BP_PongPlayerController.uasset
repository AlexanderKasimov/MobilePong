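; Player controller for a touch-screen Pong game that switches between menu, one-player and two-player modes.
; Mode functions swap the menu and gameplay widgets, and others handle pause, win screen and input blocking.
; Touches are deprojected to world space as paddle targets: one player drives the right paddle, while two-player touches pick a paddle by Y, ignoring a central dead zone.
; Android Back backs out of menus or toggles pause.
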(event Input|KeyboardEvents|AndroidBack
  (params (Key :type Key%20Structure))
  (:Pressed
    (switch Utilities|FlowControl|Switch|SwitchonEnum_PlayMode (Variables|Default|GetPlayMode)
      (:NewEnumerator0
        (Class|WidgetNavigation|Back(Message) (Class|ContentWidget|GetContent (Variables|/Game/UI/NewWidgets/Base_Menu.Base_Menu_C|GetMenuSlot (Variables|Default|GetNewMenuWidgetRef)))))
      (:NewEnumerator1
        (if (Game|IsGamePaused) :!label _label
          (bind _asui_gamplay_pause (Utilities|Casting|CastToUI_Gamplay_Pause (Class|ContentWidget|GetContent (Variables|/Game/UI/NewWidgets/UI_Gamplay_Base.UI_Gamplay_Base_C|GetWidgetSlot (Variables|Default|GetNewNewGameplayWidgetRef)))))
          (Default|ResumeGame _asui_gamplay_pause)
          (else
            (bind _asui_gamplay_game (Utilities|Casting|CastToUI_Gamplay_Game (Class|ContentWidget|GetContent (Variables|/Game/UI/NewWidgets/UI_Gamplay_Base.UI_Gamplay_Base_C|GetWidgetSlot (Variables|Default|GetNewNewGameplayWidgetRef)))))
            (Default|PauseGame _asui_gamplay_game))))
      (:NewEnumerator2
        (goto _label)))))

(event Input|TouchEvents|InputTouch
  (params (Location :type Vector) (FingerIndex :type ETouchIndex%20Enum))
  (bind (_locationx _locationy) (Class|PlayerController|GetInputTouchState "Touch2"))
  (bind (_locationx_2 _locationy_2) (Class|PlayerController|GetInputTouchState "Touch1"))
  (bind (_locationx_3 _locationy_3) (Class|PlayerController|GetInputTouchState "Touch1"))
  (bind _self self)
  (bind _self_2 self)
  (bind _returnvalue (Math|Vector2D|MakeVector2D _locationx _locationy))
  (bind _returnvalue_2 (Math|Vector2D|MakeVector2D _locationx_2 _locationy_2))
  (bind _worldposition (Class|GameplayStatics|DeprojectScreentoWorld _self_2 _returnvalue_2))
  (bind _worldposition_2 (Class|GameplayStatics|DeprojectScreentoWorld _self _returnvalue))
  (bind _y (Math|Vector|BreakVector _worldposition))
  (bind _y_2 (Math|Vector|BreakVector _worldposition_2))
  (:Pressed
    (switch Utilities|FlowControl|Switch|SwitchonEnum_PlayMode (Variables|Default|GetPlayMode) :!label _label
      (:NewEnumerator1
        (switch Utilities|FlowControl|Switch|SwitchonETouchIndex FingerIndex
          (:Touch1
            (Utilities|IsValid (Variables|Default|GetRightPlayerRef)
              (:Is%20Valid
                (Variables|/Game/Blueprints/BP_PlayerPaddle.BP_PlayerPaddle_C|SetTargetLocation (Variables|Default|GetRightPlayerRef) (.WorldPosition (Class|GameplayStatics|DeprojectScreentoWorld self (Math|Vector2D|MakeVector2D _locationx_3 _locationy_3)))))))))
      (:NewEnumerator2
        (switch Utilities|FlowControl|Switch|SwitchonETouchIndex FingerIndex
          (:Touch1
            (if (CallFunction|IsInputinValidZone _y) :!label _label_2
              (Variables|/Game/Blueprints/BP_PlayerPaddle.BP_PlayerPaddle_C|SetTargetLocation (select (CallFunction|IsLeftPlayerInput _y) (Variables|Default|GetLeftPlayerRef) (Variables|Default|GetRightPlayerRef)) _worldposition)))
          (:Touch2
            (Utilities|FlowControl|Sequence
              (:then_0
                (goto _label_2))
              (:then_1
                (if (CallFunction|IsInputinValidZone _y_2)
                  (Variables|/Game/Blueprints/BP_PlayerPaddle.BP_PlayerPaddle_C|SetTargetLocation (select (CallFunction|IsLeftPlayerInput _y_2) (Variables|Default|GetLeftPlayerRef) (Variables|Default|GetRightPlayerRef)) _worldposition_2)))))))))
  (:Moved
    (goto _label)))

(fn ConstructionScript)

(fn IsInputinValidZone
  (params (Y :type Float%20%28single-precision%29))
  (return (> (Math|Float|Absolute(Float) Y) (Variables|Default|GetInvalidZoneRange))))

(fn IsLeftPlayerInput
  (params (Y :type Float%20%28single-precision%29))
  (return (> Y (Variables|Default|GetInvalidZoneRange))))

(fn BlockInput
  (Input|DisableInput 0))

(fn UnBlockInput
  (Input|EnableInput 0))

(fn SetMenuMode
  (Utilities|FlowControl|Sequence
    (:then_0
      (Utilities|IsValid (Variables|Default|GetNewGameplayWidgetRef)
        (:Is%20Valid
          (Widget|RemovefromParent (Variables|Default|GetNewGameplayWidgetRef)))))
    (:then_1
      (bind _returnvalue (UserInterface|CreateWidget "/Game/UI/NewWidgets/Base_Menu.Base_Menu_C"))
      (bind _output_get (Variables|Default|SetNewMenuWidgetRef _returnvalue))
      (UserInterface|Viewport|AddtoViewport _output_get 0)
      (Default|SetMainMenu (Variables|Default|GetNewMenuWidgetRef))
      (Variables|Default|SetPlayMode "NewEnumerator0"))))

(fn Set1PMode
  (Widget|RemovefromParent (Variables|Default|GetNewMenuWidgetRef))
  (Utilities|FlowControl|Sequence
    (:then_0
      ;[1 1 1] ?
      (Utilities|IsValid (Variables|Default|GetNewGameplayWidgetRef)
        (:Is%20Valid
          (Widget|RemovefromParent (Variables|Default|GetNewGameplayWidgetRef)))))
    (:then_1
      (bind _returnvalue (UserInterface|CreateWidget "/Game/UI/NewWidgets/UI_Gamplay_Base.UI_Gamplay_Base_C"))
      (Variables|Default|SetNewNewGameplayWidgetRef _returnvalue)
      (Default|SetGameUI _returnvalue)
      (UserInterface|Viewport|AddtoViewport _returnvalue 0)
      (Variables|Default|SetPlayMode "NewEnumerator1"))))

(fn SetWinScreenMode
  (params (WinnerText :type Text))
  (Default|CreateWinscreenWidget (Variables|Default|GetNewNewGameplayWidgetRef) WinnerText))

(fn SetPauseMode
  (Game|SetGamePaused true))

(fn SetUnPauseMode
  (Game|SetGamePaused false))

(fn Set2PMode
  (Widget|RemovefromParent (Variables|Default|GetNewMenuWidgetRef))
  (Utilities|FlowControl|Sequence
    (:then_0
      (Utilities|IsValid (Variables|Default|GetNewGameplayWidgetRef)
        (:Is%20Valid
          (Widget|RemovefromParent (Variables|Default|GetNewGameplayWidgetRef)))))
    (:then_1
      (bind _returnvalue (UserInterface|CreateWidget "/Game/UI/NewWidgets/UI_Gamplay_Base.UI_Gamplay_Base_C"))
      (bind _output_get (Variables|Default|SetNewNewGameplayWidgetRef _returnvalue))
      (Default|SetGameUI _output_get)
      (UserInterface|Viewport|AddtoViewport _output_get 0)
      (Variables|Default|SetPlayMode "NewEnumerator2"))))