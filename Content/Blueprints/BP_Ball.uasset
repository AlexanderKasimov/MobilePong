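; BP_Ball is the Pong ball, which hands itself to the AI paddle on BeginPlay and moves each Tick by a swept SetActorLocation along its direction.
; Blocking hits branch on the hit actor's BP_ObjectType component: bounds flip vertical direction, while paddles reverse horizontal direction and skew the bounce by hit offset from paddle center.
; Goal hits report the border side to GM_BasePong, then destroy the ball.
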(event EventBeginPlay
  (bind _outactors (Actor|GetAllActorsOfClass "/Game/Blueprints/BP_PaddleAI.BP_PaddleAI_C"))
  (Variables|/Game/Blueprints/BP_PaddleAI.BP_PaddleAI_C|SetBallRef (Utilities|Array|Get(acopy) _outactors) self))

(event Collision|EventActorBeginOverlap
  (params (OtherActor :type Actor%20Object%20Reference)))

(event EventTick
  (params (DeltaSeconds :type Float%20%28single-precision%29))
  (bind _sweephitresult (Transformation|SetActorLocation (+ (* (Math|Vector|Normalize (Variables|Default|GetDirection)) (Variables|Default|GetVelocity)) (Transformation|GetActorLocation)) true false))
  (if (.bBlockingHit (Collision|BreakHitResult _sweephitresult))
    (Utilities|IsValid (Actor|GetComponentbyClass (.HitActor (Collision|BreakHitResult _sweephitresult)) "/Game/Blueprints/BP_ObjectType.BP_ObjectType_C")
      (:Is%20Valid
        (switch Utilities|FlowControl|Switch|SwitchonEnum_ObjectType (Variables|/Game/Blueprints/BP_ObjectType.BP_ObjectType_C|GetObjectType (Actor|GetComponentbyClass (.HitActor (Collision|BreakHitResult _sweephitresult)) "/Game/Blueprints/BP_ObjectType.BP_ObjectType_C"))
          (:NewEnumerator0
            (Variables|Default|SetDirection (Math|Vector|MakeVector (.X (Math|Vector|BreakVector (Variables|Default|GetDirection))) (.Y (Math|Vector|BreakVector (Variables|Default|GetDirection))) (* (.Z (Math|Vector|BreakVector (Variables|Default|GetDirection))) -1.0))))
          (:NewEnumerator2
            (Variables|Default|SetDirection (Math|Vector|MakeVector (.X (Math|Vector|BreakVector (Variables|Default|GetDirection))) (* (.Y (Math|Vector|BreakVector (Variables|Default|GetDirection))) -1.0) (+ (.Z (Math|Vector|BreakVector (Variables|Default|GetDirection))) (* (Math|Float|MapRangeClamped (.Z (Math|Vector|BreakVector (- (Transformation|GetActorLocation) (Transformation|GetActorLocation (.HitActor (Collision|BreakHitResult _sweephitresult)))))) -5e+01 5e+01 -1.0 1.0) (Variables|Default|GetBounceAngle))))))
          (:NewEnumerator1
            (Utilities|FlowControl|Sequence
              (:then_0
                (bind _asgm_base_pong (Utilities|Casting|CastToGM_BasePong (Game|GetGameMode)))
                (Default|PaddleScored _asgm_base_pong (Variables|/Game/Blueprints/BP_ObjectType.BP_ObjectType_C|GetisLeftBorder? (Actor|GetComponentbyClass (.HitActor (Collision|BreakHitResult _sweephitresult)) "/Game/Blueprints/BP_ObjectType.BP_ObjectType_C"))))
              (:then_1
                (Actor|DestroyActor)))))))))

(fn ConstructionScript
  (Transformation|SetRelativeRotation (Variables|Default|GetPaperSprite) "0,90.000000, 0" false false))